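; BP_AutoPilar is a building helper actor that procedurally lays out a row of static meshes, likely pillars with optional wall sections, along a line.
; Its construction script normalizes the WallEnd vector for direction and adds a mesh every 300 units along its length.
; IsWall adds a second mesh at each step, and one more mesh follows the loop to close the row.
; The event graph is empty.
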(fn `UserConstructionScript`
  (bind _wallend (`self.WallEnd`))
  (bind _walldirection (`self.WallDirection`))
  (set `self.WallDirection` (`KismetMathLibrary.Normal` _wallend))
  (for _index (range (+ (`KismetMathLibrary.FTrunc` (/ (`KismetMathLibrary.VSize` _wallend) 300.0)) 1))
    (bind _returnvalue (* _walldirection _index 300))
    (`AddComponent|NODE_AddStaticMeshComponent-0` :`RelativeTransform` (`KismetMathLibrary.MakeTransform` _returnvalue))
    (if (`self.is_wall`)
      (`AddComponent|NODE_AddStaticMeshComponent-1` :`RelativeTransform` (`KismetMathLibrary.MakeTransform` _returnvalue))))
  (`AddComponent|NODE_AddStaticMeshComponent-2` :`RelativeTransform` (`KismetMathLibrary.MakeTransform` (* _walldirection _index 300))))