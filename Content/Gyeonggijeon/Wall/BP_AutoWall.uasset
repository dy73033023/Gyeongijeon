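; BP_AutoWall is a procedural wall actor in the Gyeonggijeon content, built from repeated static mesh segments.
; Its Construction Script adds mesh components every 20 units from the actor's origin along the WallEnd vector, with the count derived from that vector's length.
; Each segment takes its rotation from the normalized wall direction and keeps unit scale.
; The Event Graph holds only disabled placeholder events, so it has no runtime logic.
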(fn `UserConstructionScript`
  (bind _wallend (`self.WallEnd`))
  (bind _walldirection (`self.WallDirection`))
  (set `self.WallDirection` (`KismetMathLibrary.Normal` _wallend))
  (for _index (range (+ (`KismetMathLibrary.FTrunc` (/ (`KismetMathLibrary.VSize` _wallend) 20.0)) 1))
    (`AddComponent|NODE_AddStaticMeshComponent-0` :`RelativeTransform` (`KismetMathLibrary.MakeTransform` (* _index 20 _walldirection) (`KismetMathLibrary.ComposeRotators` (`KismetMathLibrary.Conv_VectorToRotator` _walldirection) (`KismetMathLibrary.MakeRotator` 0.0)) (1.0 1.0 0.0)))))