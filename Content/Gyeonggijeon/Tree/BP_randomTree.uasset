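; Random tree actor that varies its appearance through the Construction Script, with no active runtime logic.
; Two nested, independent random rolls pick one of three Add Static Mesh Component nodes, so the branches have unequal odds.
; The chosen component is placed at the Pos variable with a random yaw and a random non-uniform downscale.
; Randomness is unseeded, so each construction rerun rerolls the result.
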(fn `UserConstructionScript`
  (bind _returnvalue (`KismetMathLibrary.RandomIntegerInRange` 0 2))
  (bind _returnvalue_2 (`KismetMathLibrary.RandomFloatInRange` 0.0 360.0))
  (bind _returnvalue_3 (`KismetMathLibrary.RandomFloatInRange` 0.5 0.7))
  (bind _output_get (set `self.scale` (`KismetMathLibrary.MakeVector` _returnvalue_3 _returnvalue_3 _returnvalue_3)))
  (if (== _returnvalue 0)
    (`AddComponent|NODE_AddStaticMeshComponent-2` :`RelativeTransform` (`KismetMathLibrary.MakeTransform` (`self.pos`) (`KismetMathLibrary.MakeRotator` 0.0 0.0 _returnvalue_2) _output_get))
    (elif (== _returnvalue 1)
      (`AddComponent|NODE_AddStaticMeshComponent-1` :`RelativeTransform` (`KismetMathLibrary.MakeTransform` (`self.pos`) (`KismetMathLibrary.MakeRotator` 0.0 0.0 _returnvalue_2) _output_get))
      (else
        (`AddComponent|NODE_AddStaticMeshComponent-0` :`RelativeTransform` (`KismetMathLibrary.MakeTransform` (`self.pos`) (`KismetMathLibrary.MakeRotator` 0.0 0.0 _returnvalue_2) _output_get))))))