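; BP_AutoLantern lines a wall with static meshes and BP_Light actors, then lights them in sequence during play.
; The construction script places scaled meshes along the WallEnd direction, with the count derived from that vector's length.
; BeginPlay spawns and stores as many lights, but along world X at slightly tighter spacing than the meshes.
; Tick turns on the next stored light about every second, with no bound on the index.
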(event `self.ReceiveBeginPlay`
  (for _index (range (+ (`KismetMathLibrary.FTrunc` (/ (`KismetMathLibrary.VSize` (`self.WallEnd`)) 210.0)) 1))
    (bind _returnvalue (`|SpawnActorFromClass` "/Game/Gyeonggijeon/Building/lantern/BP_Light.BP_Light_C" (`KismetMathLibrary.MakeTransform` (+ (`self.K2_GetActorLocation`) (`KismetMathLibrary.MakeVector` (* _index 210)))) "Undefined" "MultiplyWithRoot" null null))
    (`KismetArrayLibrary.Array_Add` (`self.NewVar`) _returnvalue)))

(event `self.ReceiveTick`
  (params (DeltaSeconds :type "Float (single-precision)"))
  (set `self.timer` (+ (`self.timer`) DeltaSeconds))
  (if (> (`self.timer`) 1.0)
    (set `self.timer` 0.0)
    (`/Game/Gyeonggijeon/Building/lantern/BPI_lantern.TurnOn` (`|GetArrayItem` (`self.NewVar`) (`self.idx`)))
    (bind _result (`/Engine/EditorBlueprintResources/StandardMacros.IncrementInt` (`self.idx`))
      (:`  `
        (set `self.idx` _result)))))

(fn `UserConstructionScript`
  (bind _wallend (`self.WallEnd`))
  (set `self.WallDirection` (`KismetMathLibrary.Normal` _wallend))
  (for _index (range (+ (`KismetMathLibrary.FTrunc` (/ (`KismetMathLibrary.VSize` _wallend) 210.0)) 1))
    (`AddComponent|NODE_AddStaticMeshComponent-1` :`RelativeTransform` (`KismetMathLibrary.MakeTransform` (* (`self.WallDirection`) _index 215) (struct) (3.0 3.0 3.0)))))